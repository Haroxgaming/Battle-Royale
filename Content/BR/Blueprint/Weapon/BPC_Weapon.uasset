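; BPC_Weapon is a Blueprint that holds a weapon's stats: magazine capacity, current munition, damage and fire rate.
; BeginPlay sets the base values and fills munition to the maximum.
; An Upgrade event raises damage, fire rate and maximum munition by fixed increments, leaving current munition unchanged.
; The graph holds only this state, with no firing or reload logic.
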(event `self.ReceiveBeginPlay`
  (bind _output_get (set `self.MunitionMax` 15))
  (set `self.Munition` _output_get)
  (set `self.Damage` 12)
  (set `self.Fire rate` 2.0))

(event `Upgrade`
  (set `self.Damage` (+ (`self.Damage`) 3))
  (set `self.Fire rate` (+ (`self.Fire rate`) 0.75))
  (set `self.MunitionMax` (+ (`self.MunitionMax`) 5)))