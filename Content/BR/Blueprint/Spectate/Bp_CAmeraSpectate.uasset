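; Spectator camera pawn that flies freely over the match and lets the player pick an AI character to follow.
; On BeginPlay it switches to flying, shows the cursor, adds the camera input context and creates the spectate widget.
; Enhanced Input drives horizontal and vertical movement.
; A left-click cursor trace selects and flags a Bp_MainIA and switches the widget page, while Spectate and BackFocusCamera blend the view between target and camera.
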(event `self.ReceiveBeginPlay`
  (`CharacterMovementComponent.SetMovementMode` (`self.CharacterMovement`) "MOVE_Flying" 0)
  (bind _asplayer_controller (cast `PlayerController` (`self.GetController`)))
  (set `PlayerController.bShowMouseCursor` true _asplayer_controller)
  (`EnhancedInputSubsystemInterface.AddMappingContext` (pcsubsystem `EnhancedInputLocalPlayerSubsystem` _asplayer_controller) "/Game/BR/Blueprint/Spectate/Input/IMC_Camera.IMC_Camera" 0 (struct))
  (bind _returnvalue (`|CreateWidget` "/Game/BR/Widget/WBP_SpectateInterafce.WBP_SpectateInterafce_C" null self))
  (bind _output_get (set `self.RefWidgetInterface` _returnvalue))
  (`UserWidget.AddToViewport` _output_get 0))

(event `Spectate`
  (`PlayerController.SetViewTargetWithBlend` (`GameplayStatics.GetPlayerController` 0) (`self.Main IA Focus`) 1.0 "VTBlend_Linear" 0.0 false))

(event `EnhancedInput|/Game/BR/Blueprint/Spectate/Input/IA_MoveCamera`
  (params (ActionValue :type "Vector2D Structure") (ElapsedSeconds :type "Float (double-precision)") (TriggeredSeconds :type "Float (double-precision)") (InputAction :type "InputAction Object Reference" :default "/Game/BR/Blueprint/Spectate/Input/IA_MoveCamera.IA_MoveCamera"))
  (:`Triggered`
    (`self.AddMovementInput` (* (`self.GetActorForwardVector`) 1000.0) ActionValue_X)
    (`self.AddMovementInput` (* (`self.GetActorRightVector`) 1500.0) ActionValue_Y)))

(event `BackFocusCamera`
  (`PlayerController.SetViewTargetWithBlend` (`GameplayStatics.GetPlayerController` 0) self 1.0 "VTBlend_Linear" 0.0 false))

(event `EnhancedInput|/Game/BR/Blueprint/Spectate/Input/IA_Down`
  (params (ActionValue :type Boolean) (ElapsedSeconds :type "Float (double-precision)") (TriggeredSeconds :type "Float (double-precision)") (InputAction :type "InputAction Object Reference" :default "/Game/BR/Blueprint/Spectate/Input/IA_Down.IA_Down"))
  (:`Triggered`
    (`self.AddMovementInput` (* (`SceneComponent.GetForwardVector` (`self.Arrow1`)) 2000.0) -1.0)))

(event `EnhancedInput|/Game/BR/Blueprint/Spectate/Input/IA_Up`
  (params (ActionValue :type Boolean) (ElapsedSeconds :type "Float (double-precision)") (TriggeredSeconds :type "Float (double-precision)") (InputAction :type "InputAction Object Reference" :default "/Game/BR/Blueprint/Spectate/Input/IA_Up.IA_Up"))
  (:`Triggered`
    (`self.AddMovementInput` (* (`SceneComponent.GetForwardVector` (`self.Arrow1`)) 2000.0))))

(event `Key|LeftMouseButton`
  (params (Key :type "Key Structure"))
  (bind (_worldlocation _worlddirection) (`PlayerController.DeprojectMousePositionToWorld` (`GameplayStatics.GetPlayerController` 0)))
  (:`Pressed`
    (bind (_outhit _returnvalue) (`KismetSystemLibrary.LineTraceSingle` (`self.K2_GetActorLocation`) (+ _worldlocation (* _worlddirection 6000.0)) "TraceTypeQuery1"))
    (if _returnvalue
      (bind _asbp_main_ia (cast `/Game/BR/Blueprint/IA/Bp_MainIA` (`.HitActor` (`GameplayStatics.BreakHitResult` _outhit))))
      (bind _output_get (set `self.Main IA Focus` _asbp_main_ia))
      (`WidgetSwitcher.SetActiveWidgetIndex` (`/Game/BR/Widget/WBP_SpectateInterafce.WidgetSwitcher` (`self.RefWidgetInterface`)) 1)
      (set `/Game/BR/Blueprint/IA/Bp_MainIA.IsSpectate?` true _output_get))))

(fn `UserConstructionScript`)