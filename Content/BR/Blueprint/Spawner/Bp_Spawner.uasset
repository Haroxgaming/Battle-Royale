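; Spawner actor that creates one Bp_MainIA AI pawn running BT_MainIA, slightly above its own transform, on BeginPlay.
; Each spawned AI gets a random behavior type (Passif, Normal or Agressif), which also picks the material on its mesh.
; It draws a random name from the TabName list on the player's Bp_CameraSpectate character, then removes it from that list so later spawns do not reuse it.
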(event `self.ReceiveBeginPlay`
  (bind _returnvalue (`self.GetTransform`))
  (bind _tabname (`/Game/BR/Blueprint/Spectate/Bp_CAmeraSpectate.TabName` (cast `/Game/BR/Blueprint/Spectate/Bp_CAmeraSpectate` (`GameplayStatics.GetPlayerCharacter` 0) :!pure true)))
  (bind _returnvalue_2 (`AIBlueprintHelperLibrary.SpawnAIFromClass` "/Game/BR/Blueprint/IA/Bp_MainIA.Bp_MainIA_C" "/Game/BR/Blueprint/IA/BT_MainIA.BT_MainIA" (`KismetMathLibrary.MakeVector` (.x (.location _returnvalue)) (.y (.location _returnvalue)) (+ (.z (.location _returnvalue)) 90.0)) (.rotation _returnvalue) true null))
  (bind _asbp_main_ia (cast `/Game/BR/Blueprint/IA/Bp_MainIA` _returnvalue_2 :!pure true))
  (bind _output_get (set `/Game/BR/Blueprint/IA/Bp_MainIA.TypeIA` (`KismetArrayLibrary.Array_Random` (`|MakeArray` "NewEnumerator0" "NewEnumerator1" "NewEnumerator2" :!type "/Game/BR/Blueprint/IA/E_IaType Enum")) _asbp_main_ia))
  (`PrimitiveComponent.SetMaterial` (`Character.Mesh` _asbp_main_ia) 0 (select `/Game/BR/Blueprint/IA/E_IaType` _output_get :`NewEnumerator0` "/Engine/MapTemplates/Materials/BasicAsset03.BasicAsset03" :`NewEnumerator1` "/Engine/MapTemplates/Materials/BasicAsset02.BasicAsset02" :`NewEnumerator2` "/Engine/MapTemplates/Materials/BasicAsset01.BasicAsset01" :!type "MaterialInterface Object Reference"))
  (bind _output_get_2 (set `/Game/BR/Blueprint/IA/Bp_MainIA.IaName` (`KismetArrayLibrary.Array_Random` _tabname) _asbp_main_ia))
  (`KismetArrayLibrary.Array_RemoveItem` _tabname _output_get_2))

(fn `UserConstructionScript`)