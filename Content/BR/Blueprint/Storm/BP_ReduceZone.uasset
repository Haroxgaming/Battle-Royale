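; Battle royale storm zone actor that shrinks in three phases and damages AI characters (Bp_MainIA) that leave it.
; Looping timers step Diametre down to rescale the static mesh, each phase shrinking faster with higher damage, separated by timed waits.
; Capsule end overlap starts storm damage at the current phase's value and begin overlap stops it, with IsInZone set true outside the capsule.
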(event `self.ReceiveBeginPlay`
  ;[1 1 1] first reduce
  (set `self.Damage` 2.0)
  (bind _returnvalue (`KismetSystemLibrary.K2_SetTimerDelegate` (delegate `First reduce`) 0.05 true))
  (set `self.Event first reduce` _returnvalue))

(event `Second reduce`
  ;[1 1 1] Second reduce
  (set `self.Damage` 5.0)
  (bind _returnvalue (`KismetSystemLibrary.K2_SetTimerDelegate` (delegate `Reduce second`) 0.05 true))
  (set `self.Event second reduce` _returnvalue))

(event `Reduce last`
  ;[1 1 1] Third reduce
  (set `self.Damage` 10.0)
  (bind _returnvalue (`KismetSystemLibrary.K2_SetTimerDelegate` (delegate `Third reduce`) 0.05 true))
  (set `self.Event third reduce` _returnvalue))

(event `First reduce`
  (bind _diametre (`self.Diametre`))
  ;[1 1 1] first reduce
  (bind _output_get (set `self.Diametre` (- (`self.Diametre`) 0.05)))
  (if (not (<= _output_get 90.0))
    (`SceneComponent.SetRelativeScale3D` (`self.StaticMesh`) (`KismetMathLibrary.MakeVector` _diametre _diametre 150.0))
    (else
      (`KismetSystemLibrary.K2_ClearAndInvalidateTimerHandle` (`self.Event first reduce`))
      (bind _returnvalue (`KismetSystemLibrary.K2_SetTimerDelegate` (delegate `EndWaitZone`) 20.0))
      (set `self.TimerZone` _returnvalue))))

(event `Reduce second`
  (bind _diametre (`self.Diametre`))
  ;[1 1 1] Second reduce
  (bind _output_get (set `self.Diametre` (- (`self.Diametre`) 0.1)))
  (if (not (<= _output_get 60.0))
    (`SceneComponent.SetRelativeScale3D` (`self.StaticMesh`) (`KismetMathLibrary.MakeVector` _diametre _diametre 150.0))
    (else
      (`KismetSystemLibrary.K2_ClearAndInvalidateTimerHandle` (`self.Event second reduce`))
      (`KismetSystemLibrary.Delay` 10.0)
      (`self.Reduce last`))))

(event `Third reduce`
  (bind _diametre (`self.Diametre`))
  ;[1 1 1] Third reduce
  (bind _output_get (set `self.Diametre` (- (`self.Diametre`) 0.2)))
  (if (not (<= _output_get 10.0))
    (`SceneComponent.SetRelativeScale3D` (`self.StaticMesh`) (`KismetMathLibrary.MakeVector` _diametre _diametre 150.0))
    (else
      (`KismetSystemLibrary.K2_ClearAndInvalidateTimerHandle` (`self.Event third reduce`)))))

(event `EndWaitZone`
  ;[1 1 1] first reduce
  (`self.Second reduce`))

(event `self.Capsule.OnComponentEndOverlap`
  (params (OverlappedComponent :type "PrimitiveComponent Object Reference") (OtherActor :type "Actor Object Reference") (OtherComp :type "PrimitiveComponent Object Reference") (OtherBodyIndex :type Integer))
  ;[1 1 1] Storm damage
  (bind _asbp_main_ia (cast `/Game/BR/Blueprint/IA/Bp_MainIA` OtherActor))
  (`/Game/BR/Blueprint/IA/Bp_MainIA.In storm` _asbp_main_ia (`self.Damage`) self)
  (set `/Game/BR/Blueprint/IA/Bp_MainIA.IsInZone?` true _asbp_main_ia)
  (`KismetSystemLibrary.PrintString` "iN"))

(event `self.Capsule.OnComponentBeginOverlap`
  (params (OverlappedComponent :type "PrimitiveComponent Object Reference") (OtherActor :type "Actor Object Reference") (OtherComp :type "PrimitiveComponent Object Reference") (OtherBodyIndex :type Integer) (bFromSweep :type Boolean) (SweepResult :type "HitResult Structure (by ref)"))
  ;[1 1 1] Storm damage
  (bind _asbp_main_ia (cast `/Game/BR/Blueprint/IA/Bp_MainIA` OtherActor))
  (`/Game/BR/Blueprint/IA/Bp_MainIA.stop strom domage` _asbp_main_ia)
  (set `/Game/BR/Blueprint/IA/Bp_MainIA.IsInZone?` false _asbp_main_ia))

(fn `UserConstructionScript`)