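; Behavior Tree task that moves a Bp_MainIA pawn to a blackboard zone location, finishing when the move ends.
; In parallel, a 2-second timer re-arms while IsInZone is true; otherwise it finishes the task, occasionally dashing and resetting zone focus first.
; The looping VerifZone timer is cleared immediately after creation, so the 2-second check does the polling.
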(event `VerifZone`
  (if (not (`/Game/BR/Blueprint/IA/Bp_MainIA.IsInZone?` (stale `self.ReceiveExecuteAI` _asbp_main_ia)))
    (`KismetSystemLibrary.K2_ClearAndInvalidateTimerHandle` (stale `self.ReceiveExecuteAI` _returnvalue) :!label _label)
    (`KismetSystemLibrary.K2_SetTimerDelegate` (delegate `TimerToStopFocus`) 2.0 :!label _label_2)
    (`KismetSystemLibrary.PrintString` "InZone")
    (else
      (`KismetSystemLibrary.PrintString` "TryZone"))))

(event `TimerToStopFocus`
  (if (`/Game/BR/Blueprint/IA/Bp_MainIA.IsInZone?` (stale `self.ReceiveExecuteAI` _asbp_main_ia))
    (goto _label_2)
    (else
      (if (`KismetMathLibrary.RandomBoolWithWeight` 0.2)
        (`/Game/BR/Blueprint/IA/Bp_MainIA.Dash` (stale `self.ReceiveExecuteAI` _asbp_main_ia))
        (`/Game/BR/Blueprint/IA/AIC_MainIA.ResetFocusZone` (stale `self.ReceiveExecuteAI` _asaic_main_ia)))
      (`self.FinishExecute` true))))

(event `self.ReceiveExecuteAI`
  (params (OwnerController :type "AIController Object Reference") (ControlledPawn :type "Pawn Object Reference"))
  (bind _asbp_main_ia (cast `/Game/BR/Blueprint/IA/Bp_MainIA` ControlledPawn))
  (bind _asaic_main_ia (cast `/Game/BR/Blueprint/IA/AIC_MainIA` OwnerController))
  (`|ExecutionSequence`
    (:`then_0`
      (`|AIMoveTo` _asbp_main_ia (`BTFunctionLibrary.GetBlackboardValueAsVector` (`self.Key`)) null
        (:`OnSuccess`
          (`/Game/BR/Blueprint/IA/AIC_MainIA.ResetFocusZone` _asaic_main_ia)
          (`self.FinishExecute` true))
        (:`OnFail`
          (`self.FinishExecute` true))))
    (:`then_1`
      (bind _returnvalue (`KismetSystemLibrary.K2_SetTimerDelegate` (delegate `VerifZone`) (`GameplayStatics.GetWorldDeltaSeconds`) true))
      (goto _label))))