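; AIC_MainIA is an AI controller that runs the BT_MainIA behavior tree on BeginPlay and feeds it perception results.
; When AI Perception updates, only actors that cast to Bp_MainIA are considered.
; A sensed one is written to the ActorTarget blackboard key, and a lost one clears that key, whichever actor it held.
; Debug strings print on perception updates.
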(event `self.ReceiveBeginPlay`
  (`self.RunBehaviorTree` "/Game/BR/Blueprint/IA/BT_MainIA.BT_MainIA"))

(event `self.AIPerception.OnTargetPerceptionUpdated`
  (params (Actor :type "Actor Object Reference") (Stimulus :type "AIStimulus Structure"))
  (`KismetSystemLibrary.PrintString` "Vu")
  (bind _asbp_main_ia (cast `/Game/BR/Blueprint/IA/Bp_MainIA` Actor))
  (if (`.bSuccessfullySensed` (break `AIStimulus` Stimulus))
    (`KismetSystemLibrary.PrintString` "Yes")
    (`BlackboardComponent.SetValueAsObject` (`self.Blackboard`) "ActorTarget" _asbp_main_ia)
    (else
      (`BlackboardComponent.SetValueAsObject` (`self.Blackboard`) "ActorTarget" null))))

(fn `UserConstructionScript`)