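; Behavior tree task that makes a Bp_MainIA pawn shoot at or reload against the enemy in its KeyTarget blackboard key.
; With ammo left, it raises the pawn's Shoot flag and finishes after a FireRate timer.
; When empty, it plays a shotgun reload montage with CanShoot off, then refills ammo and finishes.
; An invalid enemy makes it call ResetEnemy on the AIC_MainIA controller and finish.
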(event `self.ReceiveExecuteAI`
  (params (OwnerController :type "AIController Object Reference") (ControlledPawn :type "Pawn Object Reference"))
  (bind _asaic_main_ia (cast `/Game/BR/Blueprint/IA/AIC_MainIA` OwnerController))
  (set `self.As AIC Main IA` _asaic_main_ia)
  (bind _asbp_main_ia (cast `/Game/BR/Blueprint/IA/Bp_MainIA` ControlledPawn))
  (set `self.As Bp Main IA` _asbp_main_ia)
  (bind _asbp_main_ia_2 (cast `/Game/BR/Blueprint/IA/Bp_MainIA` (`BTFunctionLibrary.GetBlackboardValueAsActor` (`self.KeyTarget`))))
  (set `self.RefEnnemyIA` _asbp_main_ia_2)
  (`self.Shoot`))

(event `Shoot`
  (bind _as_bp_main_ia (`self.As Bp Main IA`))
  (if (`KismetSystemLibrary.IsValid` (`self.RefEnnemyIA`))
    (if (not (<= (`/Game/BR/Blueprint/IA/Bp_MainIA.Ammo` (`self.As Bp Main IA`)) 0))
      (set `/Game/BR/Blueprint/IA/Bp_MainIA.Shoot?` true _as_bp_main_ia)
      (`KismetSystemLibrary.K2_SetTimerDelegate` (delegate `FireRate`) (`/Game/BR/Blueprint/IA/Bp_MainIA.FireRate` _as_bp_main_ia))
      (else
        (`self.Reload`)))
    (else
      (`/Game/BR/Blueprint/IA/AIC_MainIA.ResetEnemy` (`self.As AIC Main IA`))
      (`self.FinishExecute` true))))

(event `FireRate`
  (`self.FinishExecute` true))

(event `Reload`
  (`|PlayMontage` (`Character.Mesh` (`self.As Bp Main IA`)) "/Game/AnimStarterPack/Reload_Shotgun_Ironsights_Montage.Reload_Shotgun_Ironsights_Montage" 1.3
    (:`then`
      (set `/Game/BR/Blueprint/IA/Bp_MainIA.CanShoot?` false (`self.As Bp Main IA`)))
    (:`OnCompleted`
      (`self.EndReload`))))

(event `EndReload`
  (bind _as_bp_main_ia (`self.As Bp Main IA`))
  (set `/Game/BR/Blueprint/IA/Bp_MainIA.CanShoot?` true (`self.As Bp Main IA`))
  (set `/Game/BR/Blueprint/IA/Bp_MainIA.Ammo` (`/Game/BR/Blueprint/IA/Bp_MainIA.AmmoMaxReload` _as_bp_main_ia) _as_bp_main_ia)
  (`self.FinishExecute` true))

(event `StopShoot`
  (`KismetSystemLibrary.K2_ClearAndInvalidateTimerHandle` (`self.TimerShoot`)))