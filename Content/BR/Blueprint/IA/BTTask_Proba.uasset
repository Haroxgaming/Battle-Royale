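; Behavior tree task that picks a combat reaction for a Bp_MainIA pawn, either attacking or running away, at random based on its play style.
; It reads the pawn's TypeIA and makes a weighted roll: Passif mostly flees, Normal is an even split, and Agressif mostly attacks.
; The result sets the Attack or RunAway state on AIC_MainIA, then the task finishes successfully.
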(event `self.ReceiveExecuteAI`
  (params (OwnerController :type "AIController Object Reference") (ControlledPawn :type "Pawn Object Reference"))
  ;[1 1 1] ProbaStyleDeGameplay
  (bind _asbp_main_ia (cast `/Game/BR/Blueprint/IA/Bp_MainIA` ControlledPawn))
  (bind _asaic_main_ia (cast `/Game/BR/Blueprint/IA/AIC_MainIA` OwnerController))
  (switch `/Game/BR/Blueprint/IA/E_IaType` (`/Game/BR/Blueprint/IA/Bp_MainIA.TypeIA` _asbp_main_ia)
    (:`NewEnumerator0`
      (if (`KismetMathLibrary.RandomBoolWithWeight` 0.8)
        (`/Game/BR/Blueprint/IA/AIC_MainIA.SetRunAway` _asaic_main_ia true)
        (else
          (`/Game/BR/Blueprint/IA/AIC_MainIA.SetAttack` _asaic_main_ia true :!label _label))))
    (:`NewEnumerator1`
      (if (`KismetMathLibrary.RandomBoolWithWeight` 0.5)
        (goto _label)
        (else
          (`/Game/BR/Blueprint/IA/AIC_MainIA.SetRunAway` _asaic_main_ia true :!label _label_2))))
    (:`NewEnumerator2`
      (if (`KismetMathLibrary.RandomBoolWithWeight` 0.2)
        (goto _label_2)
        (else
          (`/Game/BR/Blueprint/IA/AIC_MainIA.SetAttack` _asaic_main_ia true)))))
  (`self.FinishExecute` true))