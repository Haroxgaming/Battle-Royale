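; BP_RandomObstacle is a spawner actor that scatters a set number of BP_obstacle actors around its position.
; On BeginPlay, a fast looping timer spawns one obstacle per tick rather than all at once, counting down NombreDobstacle.
; Each obstacle gets a random X/Y offset within a square centered on the spawner and a random yaw.
; The timer clears itself once the counter drops below zero.
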(event `self.ReceiveBeginPlay`
  (bind _returnvalue (`KismetSystemLibrary.K2_SetTimerDelegate` (delegate `Spawn obstacle`) 0.01 true))
  (set `self.Event Spawn obstacle` _returnvalue))

(event `Spawn obstacle`
  (bind (_returnvalue_x _returnvalue_y) (`KismetMathLibrary.BreakVector` (`self.K2_GetActorLocation`)))
  (bind _result (`/Engine/EditorBlueprintResources/StandardMacros.DecrementInt` (`self.Nombre d'obstacle`))
    (:`  `
      (if (not (< _result 0))
        (`|SpawnActorFromClass` "/Game/BR/Blueprint/Obstacle/BP_obstacle.BP_obstacle_C" (`KismetMathLibrary.MakeTransform` (`KismetMathLibrary.MakeVector` (`KismetMathLibrary.RandomFloatInRange` (- _returnvalue_x 1500.0) (+ _returnvalue_x 1500.0)) (`KismetMathLibrary.RandomFloatInRange` (- _returnvalue_y 1500.0) (+ _returnvalue_y 1500.0))) (`KismetMathLibrary.MakeRotator` -0.0 0.0 (`KismetMathLibrary.RandomFloatInRange` -90.0 90.0))) "Undefined" "MultiplyWithRoot" null null)
        (else
          (`KismetSystemLibrary.K2_ClearAndInvalidateTimerHandle` (`self.Event Spawn obstacle`)))))))

(fn `UserConstructionScript`)